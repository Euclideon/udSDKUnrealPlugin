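; BP_BouyantPlane is an actor that bobs up and down in place, as if floating.
; BeginPlay stores the starting location, then each Tick sets the location to that origin plus a sine wave on Z driven by game time.
; VerticalOffset acts as the wave's frequency and Height as its amplitude, with movement applied without sweep.
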(event `self.ReceiveBeginPlay`
  (set `self.StartingLocation` (`self.K2_GetActorLocation`)))

(event `self.ReceiveTick`
  (params (DeltaSeconds :type "Float (single-precision)"))
  (`self.K2_SetActorLocation` (+ (`self.StartingLocation`) (`KismetMathLibrary.MakeVector` 0.0 0.0 (* (`KismetMathLibrary.Sin` (* (`GameplayStatics.GetTimeSeconds`) (`self.VerticalOffset`))) (`self.Height`))))))

(fn `UserConstructionScript`)