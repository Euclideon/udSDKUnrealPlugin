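; BP_CubeSpawner is an actor that repeatedly spawns cubes around its own location.
; On BeginPlay it starts a looping timer at the SpawnTimer interval and stores the handle.
; SpawnCube spawns the configured Class at a random direction, offset by CubeSpawnDiameter, so spawns land on a spherical shell, not throughout its volume.
; Each spawn gets random rotation and uniform scale between MinScale and MaxScale, plus a debug print.
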(event `self.ReceiveBeginPlay`
  (bind _returnvalue (`KismetSystemLibrary.K2_SetTimerDelegate` (`|CreateDelegate` :!event `SpawnCube`) (`self.SpawnTimer`) true))
  (set `self.SpawnTimerHandle` _returnvalue))

(event `SpawnCube`
  (`KismetSystemLibrary.PrintString` "SPAWNING CUBE")
  (`|SpawnActorFromClass` (`self.Class`) (`KismetMathLibrary.MakeTransform` (+ (`self.K2_GetActorLocation`) (* (`KismetMathLibrary.RandomUnitVector`) (`self.CubeSpawnDiameter`))) (`KismetMathLibrary.RandomRotator` true) (`KismetMathLibrary.Conv_DoubleToVector` (`KismetMathLibrary.RandomFloatInRange` (`self.MinScale`) (`self.MaxScale`)))) "Undefined" "OverrideRootScale" null null))

(fn `UserConstructionScript`)