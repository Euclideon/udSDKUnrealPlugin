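; BP_Cube is a short-lived physics cube actor that is launched downward while tumbling.
; On BeginPlay it replaces the Cube component's linear velocity with a random downward speed and its angular velocity with a random-axis spin.
; A delay then destroys the actor after 20 seconds, so each cube cleans itself up.
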(event `self.ReceiveBeginPlay`
  (bind _cube (`self.Cube`))
  (`PrimitiveComponent.SetPhysicsLinearVelocity` _cube (* (`KismetMathLibrary.Vector_Down`) (`KismetMathLibrary.RandomFloatInRange` 500.0 750.0)) false "None")
  (`PrimitiveComponent.SetPhysicsAngularVelocityInRadians` _cube (* (`KismetMathLibrary.RandomUnitVector`) (`KismetMathLibrary.RandomFloatInRange` 1.0 3.0)) false "None")
  (`KismetSystemLibrary.Delay` 20.0)
  (`self.K2_DestroyActor`))

(fn `UserConstructionScript`)